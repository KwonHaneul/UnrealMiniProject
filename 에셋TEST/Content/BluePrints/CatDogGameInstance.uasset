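; Game instance for a cat-and-dog minigame game that stores the chosen side and drives flow between menus, stages and the ending.
; ChangeLevel switches on a game-state enum, either opening a level for the title, four minigame stages and ending, or swapping in side-select, stage-select and score widgets.
; It records the current state in most branches, and EndLevel routes each finished stage to the score screen with the mouse cursor shown.
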(event Custom|Change%20Level
  (params (Level :type PlayState%20Enum :default "NewEnumerator0"))
  (switch Utilities|FlowControl|Switch|SwitchonPlayState Level
    (:NewEnumerator0
      ;[1 1 1] 타이틀 화면
      (Game|OpenLevel(byName) "DemonStration")
      (Variables|Default|SetCurGameState "NewEnumerator0"))
    (:NewEnumerator3
      ;[1 1 1] 진영 선택화면
      (Viewport|RemoveAllWidgets)
      (bind _returnvalue (UserInterface|CreateWidget "/Game/UI_Widget_BP/WB_SideSelect.WB_SideSelect_C"))
      (UserInterface|Viewport|AddtoViewport _returnvalue 0)
      (Variables|Default|SetCurGameState "NewEnumerator3"))
    (:NewEnumerator4
      ;[1 1 1] 스테이지 선택화면
      (Viewport|RemoveAllWidgets)
      (bind _returnvalue_2 (UserInterface|CreateWidget "/Game/UI_Widget_BP/WB_StageSelect.WB_StageSelect_C"))
      (UserInterface|Viewport|AddtoViewport _returnvalue_2 0)
      (Variables|Default|SetCurGameState "NewEnumerator4"))
    (:NewEnumerator1
      (Game|OpenLevel(byName) "Stage1_RunRunRun") ; 1번 장애물 달리기
      (Variables|Default|SetCurGameState "NewEnumerator1"))
    (:NewEnumerator2
      (Game|OpenLevel(byName) "Stage2_BallThrow") ; 2번 공던지기(투호)
      (Variables|Default|SetCurGameState "NewEnumerator2"))
    (:NewEnumerator5
      (Game|OpenLevel(byName) "Stage3_EatFood") ; 3번?
      (Variables|Default|SetCurGameState "NewEnumerator5"))
    (:NewEnumerator6
      (Game|OpenLevel(byName) "Stage4_Bark") ; 4번?
      (Variables|Default|SetCurGameState "NewEnumerator6"))
    (:NewEnumerator7
      (Viewport|RemoveAllWidgets)
      (bind _returnvalue_3 (UserInterface|CreateWidget "/Game/UI_Widget_BP/WB_GameScore.WB_GameScore_C"))
      (UserInterface|Viewport|AddtoViewport _returnvalue_3 0)
      (Variables|Default|SetCurGameState "NewEnumerator7")
      (Variables|/Script/Engine.PlayerController|SetbShowMouseCursor (Game|GetPlayerController 0) true))
    (:NewEnumerator10
      (Game|OpenLevel(byName) "FinalStage_ending"))))

(event Custom|Select_Side
  (params (ChoosenSide :type Side%20Enum :default "NewEnumerator0"))
  ;[1 1 1] 진영 선택시 저장
  (Variables|Default|SetSide ChoosenSide))

(event Custom|End%20Level
  ;[1 1 1] 각 게임이 끝나면 점수 확인 창으로
  (Viewport|RemoveAllWidgets)
  (CallFunction|ChangeLevel "NewEnumerator7"))