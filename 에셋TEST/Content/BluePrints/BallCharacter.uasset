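; Player character that aims and throws a BP_Ball, previewing its arc while Space is held and spawning it on release.
; Left/Right adjust throw speed during aiming, while Up/Down pitch the ThrowTransform component within limits.
; Each Tick feeds a predicted projectile path into a temporary spline, then rebuilds spline meshes along roughly its first half.
; Preview and spawned ball share the same throw location and velocity.
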(event EventBeginPlay)

(event EventTick
  (params (DeltaSeconds :type Float%20%28single-precision%29))
  (Throwing|DrawPredictionSpline))

(event Input|KeyboardEvents|Up
  (params (Key :type Key%20Structure :default "None"))
  ;[1 1 1] 상하 방항키 입력 : Throw Transform 0도 ~ 90도 사이 조절
  (:Pressed
    (if (< (.pitch (Transformation|GetWorldRotation (Variables|Default|GetThrowTransform))) 9e+01)
      (Transformation|AddRelativeRotation (Variables|Default|GetThrowTransform) "5.000000, 0, 0" false false))))

(event Input|KeyboardEvents|Down
  (params (Key :type Key%20Structure :default "None"))
  ;[1 1 1] 상하 방항키 입력 : Throw Transform 0도 ~ 90도 사이 조절
  (:Pressed
    (if (> (.pitch (Transformation|GetWorldRotation (Variables|Default|GetThrowTransform))) 0.0)
      (Transformation|AddRelativeRotation (Variables|Default|GetThrowTransform) "-5.000000, 0, 0" false false))))

(event Input|KeyboardEvents|Left
  (params (Key :type Key%20Structure :default "None"))
  ;[1 1 1] 좌우 방향키 입력 : 0 ~ 1000 사이에서 던지는 속도 조절
  (:Pressed
    (Utilities|PredictionSplineValid?
      (:Is%20Valid
        (if (> (Variables|Throwing|GetThrowSpeed) 0.0)
          (Variables|Throwing|SetThrowSpeed (- (Variables|Throwing|GetThrowSpeed) 5e+01)))))))

(event Input|KeyboardEvents|Right
  (params (Key :type Key%20Structure :default "None"))
  ;[1 1 1] 좌우 방향키 입력 : 0 ~ 1000 사이에서 던지는 속도 조절
  (:Pressed
    (Utilities|PredictionSplineValid?
      (:Is%20Valid
        (if (< (Variables|Throwing|GetThrowSpeed) 1.2e+03)
          (Variables|Throwing|SetThrowSpeed (+ (Variables|Throwing|GetThrowSpeed) 5e+01)))))))

(event Input|KeyboardEvents|SpaceBar
  (params (Key :type Key%20Structure :default "None"))
  ;[1 1 1] Space bar 입력 : 눌렀을 때 가이드라인 표시, 뗐을 때 가이드라인이 사라지면서 BP_Ball 투척
  (:Pressed
    (Throwing|CreatePredictionSpline))
  (:Released
    (Utilities|PredictionSplineValid?
      (:Is%20Valid
        (Throwing|DestroyPredictionSpline)
        (Game|SpawnActorfromClass "/Game/BluePrints/BP_Ball.BP_Ball_C" (Math|Transform|MakeTransform (Utilities|ThrowLocation) "0, 0, 0" "1,1,1") "Undefined" 0 (Utilities|ThrowVelocity) 0)))))

(fn ConstructionScript)

(fn CreatePredictionSpline
  (bind _returnvalue (AddComponent|AddSplineComponent false))
  (Variables|Throwing|SetPredictionSpline _returnvalue))

(fn DestroyPredictionSpline
  (bind _predictionspline (Variables|Throwing|GetPredictionSpline)
    (:then
      (Components|DestroyComponent _predictionspline)
      (Variables|Throwing|SetPredictionSpline 0)
      (Throwing|DestroyPredictionMeshes))
    (:else)))

(fn DestroyPredictionMeshes
  (for _array_element (Variables|Throwing|GetPredictionSplineMeshes)
    (Components|DestroyComponent _array_element))
  (Utilities|Array|Clear (Variables|Throwing|GetPredictionSplineMeshes)))

(fn DrawPredictionSpline
  (Utilities|PredictionSplineValid?
    (:Is%20Valid
      (Utilities|FlowControl|Sequence
        (:then_0
          ;[1 1 1] Projectile Path 예측
          (bind _outpathpositions (Class|GameplayStatics|BlueprintPredictProjectilePathbyTraceChannel (Utilities|ThrowLocation) (Utilities|ThrowVelocity) true 2e+01 "ECC_WorldDynamic" false (Utilities|Array|MakeArray self) "None" 0.0 5e+01))
          (Spline|SetSplinePoints (Variables|Throwing|GetPredictionSpline) _outpathpositions "World" true)
          (Throwing|DestroyPredictionMeshes))
        (:then_1
          ;[1 1 1] Projectile Path에 따라 Spline 을 그림
          (for _index (range 0 (/ (Math|Float|Truncate (/ (Spline|GetSplineLength (Variables|Throwing|GetPredictionSpline)) 25.0)) 2))
            (Variables|Default|SetIndex _index)
            (bind _returnvalue (AddComponent|AddSplineMeshComponent false))
            (Utilities|Array|Add (Variables|Throwing|GetPredictionSplineMeshes) _returnvalue)
            (SplineMesh|SetStartandEnd _returnvalue (Spline|GetLocationatDistanceAlongSpline (Variables|Throwing|GetPredictionSpline) (* (Variables|Default|GetIndex) 25.0) "World") (Math|Vector|ClampVectorSize (Spline|GetTangentatDistanceAlongSpline (Variables|Throwing|GetPredictionSpline) (* (Variables|Default|GetIndex) 25.0) "World") 0.0 1e+02) (Spline|GetLocationatDistanceAlongSpline (Variables|Throwing|GetPredictionSpline) (* (+ (Variables|Default|GetIndex) 1) 25.0) "World") (Math|Vector|ClampVectorSize (Spline|GetTangentatDistanceAlongSpline (Variables|Throwing|GetPredictionSpline) (* (+ (Variables|Default|GetIndex) 1) 25.0) "World") 0.0 1e+02) true :!class /Script/Engine.SplineMeshComponent)))))))