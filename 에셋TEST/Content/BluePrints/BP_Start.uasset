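; BP_Start runs a five-stage arrow-key sequence minigame, creating its widgets at BeginPlay and starting with a timer on SpaceBar.
; Arrow presses store digits in arrays, which are combined into an integer and compared with each stage's hardcoded answer.
; Correct answers flash a stage widget and advance, ending with CatWin; DogWin is never shown.
; Wrong answers wait five seconds, then reuse Stage1-to-Stage2 flag changes in every stage.
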(event OnComponentBeginOverlap(Box)
  (params (OverlappedComponent :type Primitive%20Component%20Object%20Reference) (OtherActor :type Actor%20Object%20Reference) (OtherComp :type Primitive%20Component%20Object%20Reference) (OtherBodyIndex :type Integer) (bFromSweep :type Boolean) (SweepResult :type Hit%20Result%20Structure%20%28by%20ref%29)))

(event OnComponentEndOverlap(Box)
  (params (OverlappedComponent :type Primitive%20Component%20Object%20Reference) (OtherActor :type Actor%20Object%20Reference) (OtherComp :type Primitive%20Component%20Object%20Reference) (OtherBodyIndex :type Integer)))

(event OnComponentWake(Box)
  (params (WakingComponent :type Primitive%20Component%20Object%20Reference) (BoneName :type Name :default "None")))

(event EventBeginPlay
  ;[1 1 1] 스테이지 UI 생성
  (Utilities|FlowControl|Sequence
    (:then_0
      (bind _returnvalue (UserInterface|CreateWidget "/Game/UI_Widget_BP/EatFood/BP_Switch_UI.BP_Switch_UI_C"))
      (Variables|Default|SetSwitch_1 _returnvalue))
    (:then_1
      (bind _returnvalue_2 (UserInterface|CreateWidget "/Game/UI_Widget_BP/EatFood/BP_Switch_UI2.BP_Switch_UI2_C"))
      (Variables|Default|SetSwitch_2 _returnvalue_2))
    (:then_2
      (bind _returnvalue_3 (UserInterface|CreateWidget "/Game/UI_Widget_BP/EatFood/BP_Switch_UI3.BP_Switch_UI3_C"))
      (Variables|Default|SetSwitch_3 _returnvalue_3))
    (:then_3
      (bind _returnvalue_4 (UserInterface|CreateWidget "/Game/UI_Widget_BP/EatFood/BP_Switch_UI4.BP_Switch_UI4_C"))
      (Variables|Default|SetSwitch_4 _returnvalue_4))
    (:then_4
      (bind _returnvalue_5 (UserInterface|CreateWidget "/Game/UI_Widget_BP/EatFood/BP_Switch_UI5.BP_Switch_UI5_C"))
      (Variables|Default|SetSwitch_5 _returnvalue_5))
    (:then_5
      (bind _returnvalue_6 (UserInterface|CreateWidget "/Game/UI_Widget_BP/EatFood/BP_Switch_UI_2.BP_Switch_UI_2_C"))
      (Variables|Default|Setstage1 _returnvalue_6))
    (:then_6
      (bind _returnvalue_7 (UserInterface|CreateWidget "/Game/UI_Widget_BP/EatFood/BP_Switch_UI2_2.BP_Switch_UI2_2_C"))
      (Variables|Default|Setstage2 _returnvalue_7))
    (:then_7
      (bind _returnvalue_8 (UserInterface|CreateWidget "/Game/UI_Widget_BP/EatFood/BP_Switch_UI3_2.BP_Switch_UI3_2_C"))
      (Variables|Default|Setstage3 _returnvalue_8))
    (:then_8
      (bind _returnvalue_9 (UserInterface|CreateWidget "/Game/UI_Widget_BP/EatFood/BP_Switch_UI4_2.BP_Switch_UI4_2_C"))
      (Variables|Default|Setstage4 _returnvalue_9))
    (:then_9
      (bind _returnvalue_10 (UserInterface|CreateWidget "/Game/UI_Widget_BP/EatFood/BP_Switch_UI5_2.BP_Switch_UI5_2_C"))
      (Variables|Default|Setstage5 _returnvalue_10))
    (:then_10
      (bind _returnvalue_11 (UserInterface|CreateWidget "/Game/UI_Widget_BP/EatFood/BP_Clear.BP_Clear_C"))
      (Variables|Default|SetCat_win _returnvalue_11))
    (:then_11
      (bind _returnvalue_12 (UserInterface|CreateWidget "/Game/UI_Widget_BP/EatFood/BP_Clear_2.BP_Clear_2_C"))
      (Variables|Default|SetDog_win _returnvalue_12))
    (:then_12
      (bind _returnvalue_13 (UserInterface|CreateWidget "/Game/UI_Widget_BP/EatFood/Widget_startgame.Widget_startgame_C"))
      (bind _output_get (Variables|Default|Setstart _returnvalue_13))
      (UserInterface|Viewport|AddtoViewport _output_get 0)
      (Input|EnableInput (Game|GetPlayerController 0)))
    (:then_13
      (bind _returnvalue_14 (UserInterface|CreateWidget "/Game/UI_Widget_BP/EatFood/Widget_Fight.Widget_Fight_C"))
      (Variables|Default|Setfight _returnvalue_14))))

(event Input|KeyboardEvents|Right
  (params (Key :type Key%20Structure :default "None"))
  (bind _aruserinput (Variables|Default|GetarUserInput))
  (bind _aruserinput_2 (Variables|Default|GetarUserInput))
  (bind _input2 (Variables|Default|GetInput2))
  (bind _input3 (Variables|Default|GetInput3))
  (bind _input4 (Variables|Default|GetInput4))
  (:Pressed
    (Development|PrintText "오른쪽")
    (if (Variables|Default|GetStage1?)
      (Utilities|Array|SetArrayElem (Variables|Default|GetarUserInput) (Variables|Default|GetnIndex) 1 :!label _label)
      (if (Variables|Default|GetStage1?)
        (Development|PrintText "스테이지1")
        (bind _output_get (Variables|Default|SetnIndex (+ 1 (Variables|Default|GetnIndex))))
        (if (== _output_get 4)
          (Development|PrintText "4개 입력")
          (bind _output_get_2 (Variables|Default|SetuserAnswer (+ (* (Utilities|Array|Get(acopy) _aruserinput_2) 1000) (* (Utilities|Array|Get(acopy) _aruserinput_2 1) 100) (* (Utilities|Array|Get(acopy) _aruserinput_2 2) 10) (Utilities|Array|Get(acopy) _aruserinput_2 3))))
          (if (== 1142 _output_get_2)
            (Development|PrintText "정답")
            (Utilities|FlowControl|Sequence
              (:then_0
                (Development|PrintText "스테이지2 넘어감")
                (Variables|Default|SetStage2? true))
              (:then_1
                (Development|PrintText "스테이지1 종료")
                (Variables|Default|SetStage1? false)))
            (Utilities|FlowControl|Sequence
              (:then_0
                (Utilities|FlowControl|Sequence
                  (:then_0
                    (Widget|RemovefromParent (Variables|Default|GetSwitch_1)))
                  (:then_1
                    (UserInterface|Viewport|AddtoViewport (Variables|Default|Getstage1) 0)
                    (Utilities|FlowControl|Delay 1.0)
                    (Widget|RemovefromParent (Variables|Default|Getstage1)))))
              (:then_1
                (Utilities|FlowControl|Delay 1.0)
                (UserInterface|Viewport|AddtoViewport (Variables|Default|GetSwitch_2) 0)))
            (else
              (Development|PrintText "오답")
              (Utilities|FlowControl|Delay 5.0)
              (Utilities|FlowControl|Sequence
                (:then_0
                  (Development|PrintText "스테이지2 넘어감")
                  (Variables|Default|SetStage2? true))
                (:then_1
                  (Development|PrintText "스테이지1 종료")
                  (Variables|Default|SetStage1? false)))
              (Utilities|FlowControl|Sequence
                (:then_0
                  (Widget|RemovefromParent (Variables|Default|GetSwitch_1)))
                (:then_1
                  (Utilities|FlowControl|Delay 1.0)
                  (UserInterface|Viewport|AddtoViewport (Variables|Default|GetSwitch_2) 0))))))
        (elif (Variables|Default|GetStage2?)
          (Development|PrintText "스테이지2")
          (bind _output_get_3 (Variables|Default|SetnIndex (+ 1 (Variables|Default|GetnIndex))))
          (if (== _output_get_3 9)
            (Development|PrintText "5개 입력")
            (bind _output_get_4 (Variables|Default|SetuserAnswer (+ (* (Utilities|Array|Get(acopy) _aruserinput 4) 10000) (* (Utilities|Array|Get(acopy) _aruserinput 5) 1000) (* (Utilities|Array|Get(acopy) _aruserinput 6) 100) (* (Utilities|Array|Get(acopy) _aruserinput 7) 10) (Utilities|Array|Get(acopy) _aruserinput 8))))
            (if (== 23412 _output_get_4)
              (Development|PrintText "2스테이지 정답")
              (Utilities|FlowControl|Sequence
                (:then_0
                  (Development|PrintText "스테이지2 종료")
                  (Variables|Default|SetStage2? false))
                (:then_1
                  (Development|PrintText "스테이지3 시작")
                  (Variables|Default|SetStage3? true)))
              (Utilities|FlowControl|Sequence
                (:then_0
                  (Utilities|FlowControl|Sequence
                    (:then_0
                      (Widget|RemovefromParent (Variables|Default|GetSwitch_2)))
                    (:then_1
                      (UserInterface|Viewport|AddtoViewport (Variables|Default|Getstage2) 0)
                      (Utilities|FlowControl|Delay 1.0)
                      (Widget|RemovefromParent (Variables|Default|Getstage2)))))
                (:then_1
                  (Utilities|FlowControl|Delay 1.0)
                  (UserInterface|Viewport|AddtoViewport (Variables|Default|GetSwitch_3) 0)))
              (else
                (Development|PrintText "오답")
                (Utilities|FlowControl|Delay 5.0)
                (Utilities|FlowControl|Sequence
                  (:then_0
                    (Development|PrintText "스테이지2 넘어감")
                    (Variables|Default|SetStage2? true))
                  (:then_1
                    (Development|PrintText "스테이지1 종료")
                    (Variables|Default|SetStage1? false)))
                (Utilities|FlowControl|Sequence
                  (:then_0
                    (Widget|RemovefromParent (Variables|Default|GetSwitch_2)))
                  (:then_1
                    (Utilities|FlowControl|Delay 1.0)
                    (UserInterface|Viewport|AddtoViewport (Variables|Default|GetSwitch_3) 0))))))))
      (elif (Variables|Default|GetStage2?)
        (goto _label)
        (elif (Variables|Default|GetStage3?)
          (Utilities|Array|SetArrayElem (Variables|Default|GetInput2) (Variables|Default|GetIndex2) 1)
          (Development|PrintText "스테이지3")
          (bind _output_get_5 (Variables|Default|SetIndex2 (+ 1 (Variables|Default|GetIndex2))))
          (if (== _output_get_5 6)
            (Development|PrintText "6개 입력")
            (bind _output_get_6 (Variables|Default|SetuserAnswer (+ (* (Utilities|Array|Get(acopy) _input2) 100000) (* (Utilities|Array|Get(acopy) _input2 1) 10000) (* (Utilities|Array|Get(acopy) _input2 2) 1000) (* (Utilities|Array|Get(acopy) _input2 3) 100) (* (Utilities|Array|Get(acopy) _input2 4) 10) (Utilities|Array|Get(acopy) _input2 5))))
            (if (== 442113 _output_get_6)
              (Development|PrintText "3스테이지 정답")
              (Utilities|FlowControl|Sequence
                (:then_0
                  (Development|PrintText "스테이지3 종료")
                  (Variables|Default|SetStage3? false))
                (:then_1
                  (Development|PrintText "스테이지4 시작")
                  (Variables|Default|Setstage4? true)))
              (Utilities|FlowControl|Sequence
                (:then_0
                  (Utilities|FlowControl|Sequence
                    (:then_0
                      (Widget|RemovefromParent (Variables|Default|GetSwitch_3)))
                    (:then_1
                      (UserInterface|Viewport|AddtoViewport (Variables|Default|Getstage3) 0)
                      (Utilities|FlowControl|Delay 1.0)
                      (Widget|RemovefromParent (Variables|Default|Getstage3)))))
                (:then_1
                  (Utilities|FlowControl|Delay 1.0)
                  (UserInterface|Viewport|AddtoViewport (Variables|Default|GetSwitch_4) 0)))
              (else
                (Development|PrintText "오답")
                (Utilities|FlowControl|Delay 5.0)
                (Utilities|FlowControl|Sequence
                  (:then_0
                    (Development|PrintText "스테이지2 넘어감")
                    (Variables|Default|SetStage2? true))
                  (:then_1
                    (Development|PrintText "스테이지1 종료")
                    (Variables|Default|SetStage1? false)))
                (Utilities|FlowControl|Sequence
                  (:then_0
                    (Widget|RemovefromParent (Variables|Default|GetSwitch_3)))
                  (:then_1
                    (Utilities|FlowControl|Delay 1.0)
                    (UserInterface|Viewport|AddtoViewport (Variables|Default|GetSwitch_4) 0))))))
          (elif (Variables|Default|Getstage4?)
            (Utilities|Array|SetArrayElem (Variables|Default|GetInput3) (Variables|Default|GetIndex3) 1)
            (Development|PrintText "스테이지4")
            (bind _output_get_7 (Variables|Default|SetIndex3 (+ (Variables|Default|GetIndex3) 1)))
            (if (== _output_get_7 7)
              (Development|PrintText "7개 입력")
              (bind _output_get_8 (Variables|Default|SetuserAnswer (+ (* (Utilities|Array|Get(acopy) _input3) 1000000) (* (Utilities|Array|Get(acopy) _input3 1) 100000) (* (Utilities|Array|Get(acopy) _input3 2) 10000) (* (Utilities|Array|Get(acopy) _input3 3) 1000) (* (Utilities|Array|Get(acopy) _input3 4) 100) (* (Utilities|Array|Get(acopy) _input3 5) 10) (Utilities|Array|Get(acopy) _input3 6))))
              (Development|PrintString (Utilities|String|ToString(Integer) _output_get_8))
              (if (== 4221343 _output_get_8)
                (Development|PrintText "4스테이지 정답")
                (Utilities|FlowControl|Sequence
                  (:then_0
                    (Development|PrintText "스테이지4 종료")
                    (Variables|Default|Setstage4? false))
                  (:then_1
                    (Development|PrintText "스테이지5 시작")
                    (Variables|Default|Setstage5? true)))
                (Utilities|FlowControl|Sequence
                  (:then_0
                    (Utilities|FlowControl|Sequence
                      (:then_0
                        (Widget|RemovefromParent (Variables|Default|GetSwitch_4)))
                      (:then_1
                        (UserInterface|Viewport|AddtoViewport (Variables|Default|Getstage4) 0)
                        (Utilities|FlowControl|Delay 1.0)
                        (Widget|RemovefromParent (Variables|Default|Getstage4)))))
                  (:then_1
                    (Utilities|FlowControl|Delay 1.0)
                    (UserInterface|Viewport|AddtoViewport (Variables|Default|GetSwitch_5) 0)))
                (else
                  (Development|PrintText "4스테이지 오답")
                  (Utilities|FlowControl|Delay 5.0)
                  (Utilities|FlowControl|Sequence
                    (:then_0
                      (Development|PrintText "스테이지2 넘어감")
                      (Variables|Default|SetStage2? true))
                    (:then_1
                      (Development|PrintText "스테이지1 종료")
                      (Variables|Default|SetStage1? false)))
                  (Utilities|FlowControl|Sequence
                    (:then_0
                      (Widget|RemovefromParent (Variables|Default|GetSwitch_4)))
                    (:then_1
                      (Utilities|FlowControl|Delay 1.0)
                      (UserInterface|Viewport|AddtoViewport (Variables|Default|GetSwitch_5) 0))))))
            (elif (Variables|Default|Getstage5?)
              (Utilities|Array|SetArrayElem (Variables|Default|GetInput4) (Variables|Default|GetIndex4) 1)
              (Development|PrintText "스테이지5")
              (bind _output_get_9 (Variables|Default|SetIndex4 (+ (Variables|Default|GetIndex4) 1)))
              (if (== _output_get_9 8)
                (Development|PrintText "8개 입력")
                (bind _output_get_10 (Variables|Default|SetuserAnswer (+ (* (Utilities|Array|Get(acopy) _input4) 10000000) (* (Utilities|Array|Get(acopy) _input4 1) 1000000) (* (Utilities|Array|Get(acopy) _input4 2) 100000) (* (Utilities|Array|Get(acopy) _input4 3) 10000) (* (Utilities|Array|Get(acopy) _input4 4) 1000) (* (Utilities|Array|Get(acopy) _input4 5) 100) (* (Utilities|Array|Get(acopy) _input4 6) 10) (Utilities|Array|Get(acopy) _input4 7))))
                (if (== 12413412 _output_get_10)
                  (Development|PrintText "5스테이지 정답")
                  (Utilities|FlowControl|Sequence
                    (:then_0
                      (Widget|RemovefromParent (Variables|Default|GetSwitch_5)))
                    (:then_1
                      (UserInterface|Viewport|AddtoViewport (Variables|Default|Getstage5) 0)
                      (Utilities|FlowControl|Delay 1.0)
                      (Widget|RemovefromParent (Variables|Default|Getstage5))
                      (UserInterface|Viewport|AddtoViewport (Variables|Default|GetCat_win) 0)))
                  (else
                    (Development|PrintText "오답")
                    (Utilities|FlowControl|Delay 5.0)
                    (Utilities|FlowControl|Sequence
                      (:then_0
                        (Development|PrintText "스테이지2 넘어감")
                        (Variables|Default|SetStage2? true))
                      (:then_1
                        (Development|PrintText "스테이지1 종료")
                        (Variables|Default|SetStage1? false)))
                    (Widget|RemovefromParent (Variables|Default|Getstage5))))))))))))

(event Input|KeyboardEvents|SpaceBar
  (params (Key :type Key%20Structure :default "None"))
  (:Pressed
    (Development|PrintString "Hello")
    (Utilities|FlowControl|Sequence
      (:then_0
        (UserInterface|Viewport|AddtoViewport (Variables|Default|GetSwitch_1) 0)
        (Development|PrintString "timer")
        (bind _returnvalue (UserInterface|CreateWidget "/Game/UI_Widget_BP/EatFood/Timer.Timer_C"))
        (UserInterface|Viewport|AddtoViewport _returnvalue 0)
        (Default|CallTimerstart))
      (:then_1
        (UserInterface|Viewport|AddtoViewport (Variables|Default|Getfight) 0))
      (:then_2
        (Widget|RemovefromParent (Variables|Default|Getstart))))))

(event Input|KeyboardEvents|Left
  (params (Key :type Key%20Structure :default "None"))
  (bind _aruserinput (Variables|Default|GetarUserInput))
  (bind _aruserinput_2 (Variables|Default|GetarUserInput))
  (bind _input2 (Variables|Default|GetInput2))
  (bind _input3 (Variables|Default|GetInput3))
  (bind _input4 (Variables|Default|GetInput4))
  (:Pressed
    (Development|PrintText "왼쪽")
    (if (Variables|Default|GetStage1?)
      (Utilities|Array|SetArrayElem (Variables|Default|GetarUserInput) (Variables|Default|GetnIndex) 2 :!label _label)
      (if (Variables|Default|GetStage1?)
        (Development|PrintText "스테이지1")
        (bind _output_get (Variables|Default|SetnIndex (+ 1 (Variables|Default|GetnIndex))))
        (if (== _output_get 4)
          (Development|PrintText "4개 입력")
          (bind _output_get_2 (Variables|Default|SetuserAnswer (+ (* (Utilities|Array|Get(acopy) _aruserinput_2) 1000) (* (Utilities|Array|Get(acopy) _aruserinput_2 1) 100) (* (Utilities|Array|Get(acopy) _aruserinput_2 2) 10) (Utilities|Array|Get(acopy) _aruserinput_2 3))))
          (if (== 1142 _output_get_2)
            (Development|PrintText "정답")
            (Utilities|FlowControl|Sequence
              (:then_0
                (Development|PrintText "스테이지2 넘어감")
                (Variables|Default|SetStage2? true))
              (:then_1
                (Development|PrintText "스테이지1 종료")
                (Variables|Default|SetStage1? false)))
            (Utilities|FlowControl|Sequence
              (:then_0
                (Utilities|FlowControl|Sequence
                  (:then_0
                    (Widget|RemovefromParent (Variables|Default|GetSwitch_1)))
                  (:then_1
                    (UserInterface|Viewport|AddtoViewport (Variables|Default|Getstage1) 0)
                    (Utilities|FlowControl|Delay 1.0)
                    (Widget|RemovefromParent (Variables|Default|Getstage1)))))
              (:then_1
                (Utilities|FlowControl|Delay 1.0)
                (UserInterface|Viewport|AddtoViewport (Variables|Default|GetSwitch_2) 0)))
            (else
              (Development|PrintText "오답")
              (Utilities|FlowControl|Delay 5.0)
              (Utilities|FlowControl|Sequence
                (:then_0
                  (Development|PrintText "스테이지2 넘어감")
                  (Variables|Default|SetStage2? true))
                (:then_1
                  (Development|PrintText "스테이지1 종료")
                  (Variables|Default|SetStage1? false)))
              (Utilities|FlowControl|Sequence
                (:then_0
                  (Widget|RemovefromParent (Variables|Default|GetSwitch_1)))
                (:then_1
                  (Utilities|FlowControl|Delay 1.0)
                  (UserInterface|Viewport|AddtoViewport (Variables|Default|GetSwitch_2) 0))))))
        (elif (Variables|Default|GetStage2?)
          (Development|PrintText "스테이지2")
          (bind _output_get_3 (Variables|Default|SetnIndex (+ 1 (Variables|Default|GetnIndex))))
          (if (== _output_get_3 9)
            (Development|PrintText "5개 입력")
            (bind _output_get_4 (Variables|Default|SetuserAnswer (+ (* (Utilities|Array|Get(acopy) _aruserinput 4) 10000) (* (Utilities|Array|Get(acopy) _aruserinput 5) 1000) (* (Utilities|Array|Get(acopy) _aruserinput 6) 100) (* (Utilities|Array|Get(acopy) _aruserinput 7) 10) (Utilities|Array|Get(acopy) _aruserinput 8))))
            (if (== 23412 _output_get_4)
              (Development|PrintText "2스테이지 정답")
              (Utilities|FlowControl|Sequence
                (:then_0
                  (Development|PrintText "스테이지2 종료")
                  (Variables|Default|SetStage2? false))
                (:then_1
                  (Development|PrintText "스테이지3 시작")
                  (Variables|Default|SetStage3? true)))
              (Utilities|FlowControl|Sequence
                (:then_0
                  (Utilities|FlowControl|Sequence
                    (:then_0
                      (Widget|RemovefromParent (Variables|Default|GetSwitch_2)))
                    (:then_1
                      (UserInterface|Viewport|AddtoViewport (Variables|Default|Getstage2) 0)
                      (Utilities|FlowControl|Delay 1.0)
                      (Widget|RemovefromParent (Variables|Default|Getstage2)))))
                (:then_1
                  (Utilities|FlowControl|Delay 1.0)
                  (UserInterface|Viewport|AddtoViewport (Variables|Default|GetSwitch_3) 0)))
              (else
                (Development|PrintText "오답")
                (Utilities|FlowControl|Delay 5.0)
                (Utilities|FlowControl|Sequence
                  (:then_0
                    (Development|PrintText "스테이지2 넘어감")
                    (Variables|Default|SetStage2? true))
                  (:then_1
                    (Development|PrintText "스테이지1 종료")
                    (Variables|Default|SetStage1? false)))
                (Utilities|FlowControl|Sequence
                  (:then_0
                    (Widget|RemovefromParent (Variables|Default|GetSwitch_2)))
                  (:then_1
                    (Utilities|FlowControl|Delay 1.0)
                    (UserInterface|Viewport|AddtoViewport (Variables|Default|GetSwitch_3) 0))))))))
      (elif (Variables|Default|GetStage2?)
        (goto _label)
        (elif (Variables|Default|GetStage3?)
          (Utilities|Array|SetArrayElem (Variables|Default|GetInput2) (Variables|Default|GetIndex2) 2)
          (Development|PrintText "스테이지3")
          (bind _output_get_5 (Variables|Default|SetIndex2 (+ 1 (Variables|Default|GetIndex2))))
          (if (== _output_get_5 6)
            (Development|PrintText "6개 입력")
            (bind _output_get_6 (Variables|Default|SetuserAnswer (+ (* (Utilities|Array|Get(acopy) _input2) 100000) (* (Utilities|Array|Get(acopy) _input2 1) 10000) (* (Utilities|Array|Get(acopy) _input2 2) 1000) (* (Utilities|Array|Get(acopy) _input2 3) 100) (* (Utilities|Array|Get(acopy) _input2 4) 10) (Utilities|Array|Get(acopy) _input2 5))))
            (if (== 442113 _output_get_6)
              (Development|PrintText "3스테이지 정답")
              (Utilities|FlowControl|Sequence
                (:then_0
                  (Development|PrintText "스테이지3 종료")
                  (Variables|Default|SetStage3? false))
                (:then_1
                  (Development|PrintText "스테이지4 시작")
                  (Variables|Default|Setstage4? true)))
              (Utilities|FlowControl|Sequence
                (:then_0
                  (Utilities|FlowControl|Sequence
                    (:then_0
                      (Widget|RemovefromParent (Variables|Default|GetSwitch_3)))
                    (:then_1
                      (UserInterface|Viewport|AddtoViewport (Variables|Default|Getstage3) 0)
                      (Utilities|FlowControl|Delay 1.0)
                      (Widget|RemovefromParent (Variables|Default|Getstage3)))))
                (:then_1
                  (Utilities|FlowControl|Delay 1.0)
                  (UserInterface|Viewport|AddtoViewport (Variables|Default|GetSwitch_4) 0)))
              (else
                (Development|PrintText "오답")
                (Utilities|FlowControl|Delay 5.0)
                (Utilities|FlowControl|Sequence
                  (:then_0
                    (Development|PrintText "스테이지2 넘어감")
                    (Variables|Default|SetStage2? true))
                  (:then_1
                    (Development|PrintText "스테이지1 종료")
                    (Variables|Default|SetStage1? false)))
                (Utilities|FlowControl|Sequence
                  (:then_0
                    (Widget|RemovefromParent (Variables|Default|GetSwitch_3)))
                  (:then_1
                    (Utilities|FlowControl|Delay 1.0)
                    (UserInterface|Viewport|AddtoViewport (Variables|Default|GetSwitch_4) 0))))))
          (elif (Variables|Default|Getstage4?)
            (Utilities|Array|SetArrayElem (Variables|Default|GetInput3) (Variables|Default|GetIndex3) 2)
            (Development|PrintText "스테이지4")
            (bind _output_get_7 (Variables|Default|SetIndex3 (+ (Variables|Default|GetIndex3) 1)))
            (if (== _output_get_7 7)
              (Development|PrintText "7개 입력")
              (bind _output_get_8 (Variables|Default|SetuserAnswer (+ (* (Utilities|Array|Get(acopy) _input3) 1000000) (* (Utilities|Array|Get(acopy) _input3 1) 100000) (* (Utilities|Array|Get(acopy) _input3 2) 10000) (* (Utilities|Array|Get(acopy) _input3 3) 1000) (* (Utilities|Array|Get(acopy) _input3 4) 100) (* (Utilities|Array|Get(acopy) _input3 5) 10) (Utilities|Array|Get(acopy) _input3 6))))
              (Development|PrintString (Utilities|String|ToString(Integer) _output_get_8))
              (if (== 4221343 _output_get_8)
                (Development|PrintText "4스테이지 정답")
                (Utilities|FlowControl|Sequence
                  (:then_0
                    (Development|PrintText "스테이지4 종료")
                    (Variables|Default|Setstage4? false))
                  (:then_1
                    (Development|PrintText "스테이지5 시작")
                    (Variables|Default|Setstage5? true)))
                (Utilities|FlowControl|Sequence
                  (:then_0
                    (Utilities|FlowControl|Sequence
                      (:then_0
                        (Widget|RemovefromParent (Variables|Default|GetSwitch_4)))
                      (:then_1
                        (UserInterface|Viewport|AddtoViewport (Variables|Default|Getstage4) 0)
                        (Utilities|FlowControl|Delay 1.0)
                        (Widget|RemovefromParent (Variables|Default|Getstage4)))))
                  (:then_1
                    (Utilities|FlowControl|Delay 1.0)
                    (UserInterface|Viewport|AddtoViewport (Variables|Default|GetSwitch_5) 0)))
                (else
                  (Development|PrintText "4스테이지 오답")
                  (Utilities|FlowControl|Delay 5.0)
                  (Utilities|FlowControl|Sequence
                    (:then_0
                      (Development|PrintText "스테이지2 넘어감")
                      (Variables|Default|SetStage2? true))
                    (:then_1
                      (Development|PrintText "스테이지1 종료")
                      (Variables|Default|SetStage1? false)))
                  (Utilities|FlowControl|Sequence
                    (:then_0
                      (Widget|RemovefromParent (Variables|Default|GetSwitch_4)))
                    (:then_1
                      (Utilities|FlowControl|Delay 1.0)
                      (UserInterface|Viewport|AddtoViewport (Variables|Default|GetSwitch_5) 0))))))
            (elif (Variables|Default|Getstage5?)
              (Utilities|Array|SetArrayElem (Variables|Default|GetInput4) (Variables|Default|GetIndex4) 2)
              (Development|PrintText "스테이지5")
              (bind _output_get_9 (Variables|Default|SetIndex4 (+ (Variables|Default|GetIndex4) 1)))
              (if (== _output_get_9 8)
                (Development|PrintText "8개 입력")
                (bind _output_get_10 (Variables|Default|SetuserAnswer (+ (* (Utilities|Array|Get(acopy) _input4) 10000000) (* (Utilities|Array|Get(acopy) _input4 1) 1000000) (* (Utilities|Array|Get(acopy) _input4 2) 100000) (* (Utilities|Array|Get(acopy) _input4 3) 10000) (* (Utilities|Array|Get(acopy) _input4 4) 1000) (* (Utilities|Array|Get(acopy) _input4 5) 100) (* (Utilities|Array|Get(acopy) _input4 6) 10) (Utilities|Array|Get(acopy) _input4 7))))
                (if (== 12413412 _output_get_10)
                  (Development|PrintText "5스테이지 정답")
                  (Utilities|FlowControl|Sequence
                    (:then_0
                      (Widget|RemovefromParent (Variables|Default|GetSwitch_5)))
                    (:then_1
                      (UserInterface|Viewport|AddtoViewport (Variables|Default|Getstage5) 0)
                      (Utilities|FlowControl|Delay 1.0)
                      (Widget|RemovefromParent (Variables|Default|Getstage5))
                      (UserInterface|Viewport|AddtoViewport (Variables|Default|GetCat_win) 0)))
                  (else
                    (Development|PrintText "오답")
                    (Utilities|FlowControl|Delay 5.0)
                    (Utilities|FlowControl|Sequence
                      (:then_0
                        (Development|PrintText "스테이지2 넘어감")
                        (Variables|Default|SetStage2? true))
                      (:then_1
                        (Development|PrintText "스테이지1 종료")
                        (Variables|Default|SetStage1? false)))
                    (Widget|RemovefromParent (Variables|Default|Getstage5))))))))))))

(event Input|KeyboardEvents|Up
  (params (Key :type Key%20Structure :default "None"))
  (bind _aruserinput (Variables|Default|GetarUserInput))
  (bind _aruserinput_2 (Variables|Default|GetarUserInput))
  (bind _input2 (Variables|Default|GetInput2))
  (bind _input3 (Variables|Default|GetInput3))
  (bind _input4 (Variables|Default|GetInput4))
  (:Pressed
    (Development|PrintText "위")
    (if (Variables|Default|GetStage1?)
      (Utilities|Array|SetArrayElem (Variables|Default|GetarUserInput) (Variables|Default|GetnIndex) 3 :!label _label)
      (if (Variables|Default|GetStage1?)
        (Development|PrintText "스테이지1")
        (bind _output_get (Variables|Default|SetnIndex (+ 1 (Variables|Default|GetnIndex))))
        (if (== _output_get 4)
          (Development|PrintText "4개 입력")
          (bind _output_get_2 (Variables|Default|SetuserAnswer (+ (* (Utilities|Array|Get(acopy) _aruserinput_2) 1000) (* (Utilities|Array|Get(acopy) _aruserinput_2 1) 100) (* (Utilities|Array|Get(acopy) _aruserinput_2 2) 10) (Utilities|Array|Get(acopy) _aruserinput_2 3))))
          (if (== 1142 _output_get_2)
            (Development|PrintText "정답")
            (Utilities|FlowControl|Sequence
              (:then_0
                (Development|PrintText "스테이지2 넘어감")
                (Variables|Default|SetStage2? true))
              (:then_1
                (Development|PrintText "스테이지1 종료")
                (Variables|Default|SetStage1? false)))
            (Utilities|FlowControl|Sequence
              (:then_0
                (Utilities|FlowControl|Sequence
                  (:then_0
                    (Widget|RemovefromParent (Variables|Default|GetSwitch_1)))
                  (:then_1
                    (UserInterface|Viewport|AddtoViewport (Variables|Default|Getstage1) 0)
                    (Utilities|FlowControl|Delay 1.0)
                    (Widget|RemovefromParent (Variables|Default|Getstage1)))))
              (:then_1
                (Utilities|FlowControl|Delay 1.0)
                (UserInterface|Viewport|AddtoViewport (Variables|Default|GetSwitch_2) 0)))
            (else
              (Development|PrintText "오답")
              (Utilities|FlowControl|Delay 5.0)
              (Utilities|FlowControl|Sequence
                (:then_0
                  (Development|PrintText "스테이지2 넘어감")
                  (Variables|Default|SetStage2? true))
                (:then_1
                  (Development|PrintText "스테이지1 종료")
                  (Variables|Default|SetStage1? false)))
              (Utilities|FlowControl|Sequence
                (:then_0
                  (Widget|RemovefromParent (Variables|Default|GetSwitch_1)))
                (:then_1
                  (Utilities|FlowControl|Delay 1.0)
                  (UserInterface|Viewport|AddtoViewport (Variables|Default|GetSwitch_2) 0))))))
        (elif (Variables|Default|GetStage2?)
          (Development|PrintText "스테이지2")
          (bind _output_get_3 (Variables|Default|SetnIndex (+ 1 (Variables|Default|GetnIndex))))
          (if (== _output_get_3 9)
            (Development|PrintText "5개 입력")
            (bind _output_get_4 (Variables|Default|SetuserAnswer (+ (* (Utilities|Array|Get(acopy) _aruserinput 4) 10000) (* (Utilities|Array|Get(acopy) _aruserinput 5) 1000) (* (Utilities|Array|Get(acopy) _aruserinput 6) 100) (* (Utilities|Array|Get(acopy) _aruserinput 7) 10) (Utilities|Array|Get(acopy) _aruserinput 8))))
            (if (== 23412 _output_get_4)
              (Development|PrintText "2스테이지 정답")
              (Utilities|FlowControl|Sequence
                (:then_0
                  (Development|PrintText "스테이지2 종료")
                  (Variables|Default|SetStage2? false))
                (:then_1
                  (Development|PrintText "스테이지3 시작")
                  (Variables|Default|SetStage3? true)))
              (Utilities|FlowControl|Sequence
                (:then_0
                  (Utilities|FlowControl|Sequence
                    (:then_0
                      (Widget|RemovefromParent (Variables|Default|GetSwitch_2)))
                    (:then_1
                      (UserInterface|Viewport|AddtoViewport (Variables|Default|Getstage2) 0)
                      (Utilities|FlowControl|Delay 1.0)
                      (Widget|RemovefromParent (Variables|Default|Getstage2)))))
                (:then_1
                  (Utilities|FlowControl|Delay 1.0)
                  (UserInterface|Viewport|AddtoViewport (Variables|Default|GetSwitch_3) 0)))
              (else
                (Development|PrintText "오답")
                (Utilities|FlowControl|Delay 5.0)
                (Utilities|FlowControl|Sequence
                  (:then_0
                    (Development|PrintText "스테이지2 넘어감")
                    (Variables|Default|SetStage2? true))
                  (:then_1
                    (Development|PrintText "스테이지1 종료")
                    (Variables|Default|SetStage1? false)))
                (Utilities|FlowControl|Sequence
                  (:then_0
                    (Widget|RemovefromParent (Variables|Default|GetSwitch_2)))
                  (:then_1
                    (Utilities|FlowControl|Delay 1.0)
                    (UserInterface|Viewport|AddtoViewport (Variables|Default|GetSwitch_3) 0))))))))
      (elif (Variables|Default|GetStage2?)
        (goto _label)
        (elif (Variables|Default|GetStage3?)
          (Utilities|Array|SetArrayElem (Variables|Default|GetInput2) (Variables|Default|GetIndex2) 3)
          (Development|PrintText "스테이지3")
          (bind _output_get_5 (Variables|Default|SetIndex2 (+ 1 (Variables|Default|GetIndex2))))
          (if (== _output_get_5 6)
            (Development|PrintText "6개 입력")
            (bind _output_get_6 (Variables|Default|SetuserAnswer (+ (* (Utilities|Array|Get(acopy) _input2) 100000) (* (Utilities|Array|Get(acopy) _input2 1) 10000) (* (Utilities|Array|Get(acopy) _input2 2) 1000) (* (Utilities|Array|Get(acopy) _input2 3) 100) (* (Utilities|Array|Get(acopy) _input2 4) 10) (Utilities|Array|Get(acopy) _input2 5))))
            (if (== 442113 _output_get_6)
              (Development|PrintText "3스테이지 정답")
              (Utilities|FlowControl|Sequence
                (:then_0
                  (Development|PrintText "스테이지3 종료")
                  (Variables|Default|SetStage3? false))
                (:then_1
                  (Development|PrintText "스테이지4 시작")
                  (Variables|Default|Setstage4? true)))
              (Utilities|FlowControl|Sequence
                (:then_0
                  (Utilities|FlowControl|Sequence
                    (:then_0
                      (Widget|RemovefromParent (Variables|Default|GetSwitch_3)))
                    (:then_1
                      (UserInterface|Viewport|AddtoViewport (Variables|Default|Getstage3) 0)
                      (Utilities|FlowControl|Delay 1.0)
                      (Widget|RemovefromParent (Variables|Default|Getstage3)))))
                (:then_1
                  (Utilities|FlowControl|Delay 1.0)
                  (UserInterface|Viewport|AddtoViewport (Variables|Default|GetSwitch_4) 0)))
              (else
                (Development|PrintText "오답")
                (Utilities|FlowControl|Delay 5.0)
                (Utilities|FlowControl|Sequence
                  (:then_0
                    (Development|PrintText "스테이지2 넘어감")
                    (Variables|Default|SetStage2? true))
                  (:then_1
                    (Development|PrintText "스테이지1 종료")
                    (Variables|Default|SetStage1? false)))
                (Utilities|FlowControl|Sequence
                  (:then_0
                    (Widget|RemovefromParent (Variables|Default|GetSwitch_3)))
                  (:then_1
                    (Utilities|FlowControl|Delay 1.0)
                    (UserInterface|Viewport|AddtoViewport (Variables|Default|GetSwitch_4) 0))))))
          (elif (Variables|Default|Getstage4?)
            (Utilities|Array|SetArrayElem (Variables|Default|GetInput3) (Variables|Default|GetIndex3) 3)
            (Development|PrintText "스테이지4")
            (bind _output_get_7 (Variables|Default|SetIndex3 (+ (Variables|Default|GetIndex3) 1)))
            (if (== _output_get_7 7)
              (Development|PrintText "7개 입력")
              (bind _output_get_8 (Variables|Default|SetuserAnswer (+ (* (Utilities|Array|Get(acopy) _input3) 1000000) (* (Utilities|Array|Get(acopy) _input3 1) 100000) (* (Utilities|Array|Get(acopy) _input3 2) 10000) (* (Utilities|Array|Get(acopy) _input3 3) 1000) (* (Utilities|Array|Get(acopy) _input3 4) 100) (* (Utilities|Array|Get(acopy) _input3 5) 10) (Utilities|Array|Get(acopy) _input3 6))))
              (Development|PrintString (Utilities|String|ToString(Integer) _output_get_8))
              (if (== 4221343 _output_get_8)
                (Development|PrintText "4스테이지 정답")
                (Utilities|FlowControl|Sequence
                  (:then_0
                    (Development|PrintText "스테이지4 종료")
                    (Variables|Default|Setstage4? false))
                  (:then_1
                    (Development|PrintText "스테이지5 시작")
                    (Variables|Default|Setstage5? true)))
                (Utilities|FlowControl|Sequence
                  (:then_0
                    (Utilities|FlowControl|Sequence
                      (:then_0
                        (Widget|RemovefromParent (Variables|Default|GetSwitch_4)))
                      (:then_1
                        (UserInterface|Viewport|AddtoViewport (Variables|Default|Getstage4) 0)
                        (Utilities|FlowControl|Delay 1.0)
                        (Widget|RemovefromParent (Variables|Default|Getstage4)))))
                  (:then_1
                    (Utilities|FlowControl|Delay 1.0)
                    (UserInterface|Viewport|AddtoViewport (Variables|Default|GetSwitch_5) 0)))
                (else
                  (Development|PrintText "4스테이지 오답")
                  (Utilities|FlowControl|Delay 5.0)
                  (Utilities|FlowControl|Sequence
                    (:then_0
                      (Development|PrintText "스테이지2 넘어감")
                      (Variables|Default|SetStage2? true))
                    (:then_1
                      (Development|PrintText "스테이지1 종료")
                      (Variables|Default|SetStage1? false)))
                  (Utilities|FlowControl|Sequence
                    (:then_0
                      (Widget|RemovefromParent (Variables|Default|GetSwitch_4)))
                    (:then_1
                      (Utilities|FlowControl|Delay 1.0)
                      (UserInterface|Viewport|AddtoViewport (Variables|Default|GetSwitch_5) 0))))))
            (elif (Variables|Default|Getstage5?)
              (Utilities|Array|SetArrayElem (Variables|Default|GetInput4) (Variables|Default|GetIndex4) 3)
              (Development|PrintText "스테이지5")
              (bind _output_get_9 (Variables|Default|SetIndex4 (+ (Variables|Default|GetIndex4) 1)))
              (if (== _output_get_9 8)
                (Development|PrintText "8개 입력")
                (bind _output_get_10 (Variables|Default|SetuserAnswer (+ (* (Utilities|Array|Get(acopy) _input4) 10000000) (* (Utilities|Array|Get(acopy) _input4 1) 1000000) (* (Utilities|Array|Get(acopy) _input4 2) 100000) (* (Utilities|Array|Get(acopy) _input4 3) 10000) (* (Utilities|Array|Get(acopy) _input4 4) 1000) (* (Utilities|Array|Get(acopy) _input4 5) 100) (* (Utilities|Array|Get(acopy) _input4 6) 10) (Utilities|Array|Get(acopy) _input4 7))))
                (if (== 12413412 _output_get_10)
                  (Development|PrintText "5스테이지 정답")
                  (Utilities|FlowControl|Sequence
                    (:then_0
                      (Widget|RemovefromParent (Variables|Default|GetSwitch_5)))
                    (:then_1
                      (UserInterface|Viewport|AddtoViewport (Variables|Default|Getstage5) 0)
                      (Utilities|FlowControl|Delay 1.0)
                      (Widget|RemovefromParent (Variables|Default|Getstage5))
                      (UserInterface|Viewport|AddtoViewport (Variables|Default|GetCat_win) 0)))
                  (else
                    (Development|PrintText "오답")
                    (Utilities|FlowControl|Delay 5.0)
                    (Utilities|FlowControl|Sequence
                      (:then_0
                        (Development|PrintText "스테이지2 넘어감")
                        (Variables|Default|SetStage2? true))
                      (:then_1
                        (Development|PrintText "스테이지1 종료")
                        (Variables|Default|SetStage1? false)))
                    (Widget|RemovefromParent (Variables|Default|Getstage5))))))))))))

(event Input|KeyboardEvents|Down
  (params (Key :type Key%20Structure :default "None"))
  (bind _aruserinput (Variables|Default|GetarUserInput))
  (bind _aruserinput_2 (Variables|Default|GetarUserInput))
  (bind _input2 (Variables|Default|GetInput2))
  (bind _input3 (Variables|Default|GetInput3))
  (bind _input4 (Variables|Default|GetInput4))
  (:Pressed
    (Development|PrintText "아래")
    (if (Variables|Default|GetStage1?)
      (Utilities|Array|SetArrayElem (Variables|Default|GetarUserInput) (Variables|Default|GetnIndex) 4 :!label _label)
      (if (Variables|Default|GetStage1?)
        (Development|PrintText "스테이지1")
        (bind _output_get (Variables|Default|SetnIndex (+ 1 (Variables|Default|GetnIndex))))
        (if (== _output_get 4)
          (Development|PrintText "4개 입력")
          (bind _output_get_2 (Variables|Default|SetuserAnswer (+ (* (Utilities|Array|Get(acopy) _aruserinput_2) 1000) (* (Utilities|Array|Get(acopy) _aruserinput_2 1) 100) (* (Utilities|Array|Get(acopy) _aruserinput_2 2) 10) (Utilities|Array|Get(acopy) _aruserinput_2 3))))
          (if (== 1142 _output_get_2)
            (Development|PrintText "정답")
            (Utilities|FlowControl|Sequence
              (:then_0
                (Development|PrintText "스테이지2 넘어감")
                (Variables|Default|SetStage2? true))
              (:then_1
                (Development|PrintText "스테이지1 종료")
                (Variables|Default|SetStage1? false)))
            (Utilities|FlowControl|Sequence
              (:then_0
                (Utilities|FlowControl|Sequence
                  (:then_0
                    (Widget|RemovefromParent (Variables|Default|GetSwitch_1)))
                  (:then_1
                    (UserInterface|Viewport|AddtoViewport (Variables|Default|Getstage1) 0)
                    (Utilities|FlowControl|Delay 1.0)
                    (Widget|RemovefromParent (Variables|Default|Getstage1)))))
              (:then_1
                (Utilities|FlowControl|Delay 1.0)
                (UserInterface|Viewport|AddtoViewport (Variables|Default|GetSwitch_2) 0)))
            (else
              (Development|PrintText "오답")
              (Utilities|FlowControl|Delay 5.0)
              (Utilities|FlowControl|Sequence
                (:then_0
                  (Development|PrintText "스테이지2 넘어감")
                  (Variables|Default|SetStage2? true))
                (:then_1
                  (Development|PrintText "스테이지1 종료")
                  (Variables|Default|SetStage1? false)))
              (Utilities|FlowControl|Sequence
                (:then_0
                  (Widget|RemovefromParent (Variables|Default|GetSwitch_1)))
                (:then_1
                  (Utilities|FlowControl|Delay 1.0)
                  (UserInterface|Viewport|AddtoViewport (Variables|Default|GetSwitch_2) 0))))))
        (elif (Variables|Default|GetStage2?)
          (Development|PrintText "스테이지2")
          (bind _output_get_3 (Variables|Default|SetnIndex (+ 1 (Variables|Default|GetnIndex))))
          (if (== _output_get_3 9)
            (Development|PrintText "5개 입력")
            (bind _output_get_4 (Variables|Default|SetuserAnswer (+ (* (Utilities|Array|Get(acopy) _aruserinput 4) 10000) (* (Utilities|Array|Get(acopy) _aruserinput 5) 1000) (* (Utilities|Array|Get(acopy) _aruserinput 6) 100) (* (Utilities|Array|Get(acopy) _aruserinput 7) 10) (Utilities|Array|Get(acopy) _aruserinput 8))))
            (if (== 23412 _output_get_4)
              (Development|PrintText "2스테이지 정답")
              (Utilities|FlowControl|Sequence
                (:then_0
                  (Development|PrintText "스테이지2 종료")
                  (Variables|Default|SetStage2? false))
                (:then_1
                  (Development|PrintText "스테이지3 시작")
                  (Variables|Default|SetStage3? true)))
              (Utilities|FlowControl|Sequence
                (:then_0
                  (Utilities|FlowControl|Sequence
                    (:then_0
                      (Widget|RemovefromParent (Variables|Default|GetSwitch_2)))
                    (:then_1
                      (UserInterface|Viewport|AddtoViewport (Variables|Default|Getstage2) 0)
                      (Utilities|FlowControl|Delay 1.0)
                      (Widget|RemovefromParent (Variables|Default|Getstage2)))))
                (:then_1
                  (Utilities|FlowControl|Delay 1.0)
                  (UserInterface|Viewport|AddtoViewport (Variables|Default|GetSwitch_3) 0)))
              (else
                (Development|PrintText "오답")
                (Utilities|FlowControl|Delay 5.0)
                (Utilities|FlowControl|Sequence
                  (:then_0
                    (Development|PrintText "스테이지2 넘어감")
                    (Variables|Default|SetStage2? true))
                  (:then_1
                    (Development|PrintText "스테이지1 종료")
                    (Variables|Default|SetStage1? false)))
                (Utilities|FlowControl|Sequence
                  (:then_0
                    (Widget|RemovefromParent (Variables|Default|GetSwitch_2)))
                  (:then_1
                    (Utilities|FlowControl|Delay 1.0)
                    (UserInterface|Viewport|AddtoViewport (Variables|Default|GetSwitch_3) 0))))))))
      (elif (Variables|Default|GetStage2?)
        (goto _label)
        (elif (Variables|Default|GetStage3?)
          (Utilities|Array|SetArrayElem (Variables|Default|GetInput2) (Variables|Default|GetIndex2) 4)
          (Development|PrintText "스테이지3")
          (bind _output_get_5 (Variables|Default|SetIndex2 (+ 1 (Variables|Default|GetIndex2))))
          (if (== _output_get_5 6)
            (Development|PrintText "6개 입력")
            (bind _output_get_6 (Variables|Default|SetuserAnswer (+ (* (Utilities|Array|Get(acopy) _input2) 100000) (* (Utilities|Array|Get(acopy) _input2 1) 10000) (* (Utilities|Array|Get(acopy) _input2 2) 1000) (* (Utilities|Array|Get(acopy) _input2 3) 100) (* (Utilities|Array|Get(acopy) _input2 4) 10) (Utilities|Array|Get(acopy) _input2 5))))
            (if (== 442113 _output_get_6)
              (Development|PrintText "3스테이지 정답")
              (Utilities|FlowControl|Sequence
                (:then_0
                  (Development|PrintText "스테이지3 종료")
                  (Variables|Default|SetStage3? false))
                (:then_1
                  (Development|PrintText "스테이지4 시작")
                  (Variables|Default|Setstage4? true)))
              (Utilities|FlowControl|Sequence
                (:then_0
                  (Utilities|FlowControl|Sequence
                    (:then_0
                      (Widget|RemovefromParent (Variables|Default|GetSwitch_3)))
                    (:then_1
                      (UserInterface|Viewport|AddtoViewport (Variables|Default|Getstage3) 0)
                      (Utilities|FlowControl|Delay 1.0)
                      (Widget|RemovefromParent (Variables|Default|Getstage3)))))
                (:then_1
                  (Utilities|FlowControl|Delay 1.0)
                  (UserInterface|Viewport|AddtoViewport (Variables|Default|GetSwitch_4) 0)))
              (else
                (Development|PrintText "오답")
                (Utilities|FlowControl|Delay 5.0)
                (Utilities|FlowControl|Sequence
                  (:then_0
                    (Development|PrintText "스테이지2 넘어감")
                    (Variables|Default|SetStage2? true))
                  (:then_1
                    (Development|PrintText "스테이지1 종료")
                    (Variables|Default|SetStage1? false)))
                (Utilities|FlowControl|Sequence
                  (:then_0
                    (Widget|RemovefromParent (Variables|Default|GetSwitch_3)))
                  (:then_1
                    (Utilities|FlowControl|Delay 1.0)
                    (UserInterface|Viewport|AddtoViewport (Variables|Default|GetSwitch_4) 0))))))
          (elif (Variables|Default|Getstage4?)
            (Utilities|Array|SetArrayElem (Variables|Default|GetInput3) (Variables|Default|GetIndex3) 4)
            (Development|PrintText "스테이지4")
            (bind _output_get_7 (Variables|Default|SetIndex3 (+ (Variables|Default|GetIndex3) 1)))
            (if (== _output_get_7 7)
              (Development|PrintText "7개 입력")
              (bind _output_get_8 (Variables|Default|SetuserAnswer (+ (* (Utilities|Array|Get(acopy) _input3) 1000000) (* (Utilities|Array|Get(acopy) _input3 1) 100000) (* (Utilities|Array|Get(acopy) _input3 2) 10000) (* (Utilities|Array|Get(acopy) _input3 3) 1000) (* (Utilities|Array|Get(acopy) _input3 4) 100) (* (Utilities|Array|Get(acopy) _input3 5) 10) (Utilities|Array|Get(acopy) _input3 6))))
              (Development|PrintString (Utilities|String|ToString(Integer) _output_get_8))
              (if (== 4221343 _output_get_8)
                (Development|PrintText "4스테이지 정답")
                (Utilities|FlowControl|Sequence
                  (:then_0
                    (Development|PrintText "스테이지4 종료")
                    (Variables|Default|Setstage4? false))
                  (:then_1
                    (Development|PrintText "스테이지5 시작")
                    (Variables|Default|Setstage5? true)))
                (Utilities|FlowControl|Sequence
                  (:then_0
                    (Utilities|FlowControl|Sequence
                      (:then_0
                        (Widget|RemovefromParent (Variables|Default|GetSwitch_4)))
                      (:then_1
                        (UserInterface|Viewport|AddtoViewport (Variables|Default|Getstage4) 0)
                        (Utilities|FlowControl|Delay 1.0)
                        (Widget|RemovefromParent (Variables|Default|Getstage4)))))
                  (:then_1
                    (Utilities|FlowControl|Delay 1.0)
                    (UserInterface|Viewport|AddtoViewport (Variables|Default|GetSwitch_5) 0)))
                (else
                  (Development|PrintText "4스테이지 오답")
                  (Utilities|FlowControl|Delay 5.0)
                  (Utilities|FlowControl|Sequence
                    (:then_0
                      (Development|PrintText "스테이지2 넘어감")
                      (Variables|Default|SetStage2? true))
                    (:then_1
                      (Development|PrintText "스테이지1 종료")
                      (Variables|Default|SetStage1? false)))
                  (Utilities|FlowControl|Sequence
                    (:then_0
                      (Widget|RemovefromParent (Variables|Default|GetSwitch_4)))
                    (:then_1
                      (Utilities|FlowControl|Delay 1.0)
                      (UserInterface|Viewport|AddtoViewport (Variables|Default|GetSwitch_5) 0))))))
            (elif (Variables|Default|Getstage5?)
              (Utilities|Array|SetArrayElem (Variables|Default|GetInput4) (Variables|Default|GetIndex4) 4)
              (Development|PrintText "스테이지5")
              (bind _output_get_9 (Variables|Default|SetIndex4 (+ (Variables|Default|GetIndex4) 1)))
              (if (== _output_get_9 8)
                (Development|PrintText "8개 입력")
                (bind _output_get_10 (Variables|Default|SetuserAnswer (+ (* (Utilities|Array|Get(acopy) _input4) 10000000) (* (Utilities|Array|Get(acopy) _input4 1) 1000000) (* (Utilities|Array|Get(acopy) _input4 2) 100000) (* (Utilities|Array|Get(acopy) _input4 3) 10000) (* (Utilities|Array|Get(acopy) _input4 4) 1000) (* (Utilities|Array|Get(acopy) _input4 5) 100) (* (Utilities|Array|Get(acopy) _input4 6) 10) (Utilities|Array|Get(acopy) _input4 7))))
                (if (== 12413412 _output_get_10)
                  (Development|PrintText "5스테이지 정답")
                  (Utilities|FlowControl|Sequence
                    (:then_0
                      (Widget|RemovefromParent (Variables|Default|GetSwitch_5)))
                    (:then_1
                      (UserInterface|Viewport|AddtoViewport (Variables|Default|Getstage5) 0)
                      (Utilities|FlowControl|Delay 1.0)
                      (Widget|RemovefromParent (Variables|Default|Getstage5))
                      (UserInterface|Viewport|AddtoViewport (Variables|Default|GetCat_win) 0)))
                  (else
                    (Development|PrintText "오답")
                    (Utilities|FlowControl|Delay 5.0)
                    (Utilities|FlowControl|Sequence
                      (:then_0
                        (Development|PrintText "스테이지2 넘어감")
                        (Variables|Default|SetStage2? true))
                      (:then_1
                        (Development|PrintText "스테이지1 종료")
                        (Variables|Default|SetStage1? false)))
                    (Widget|RemovefromParent (Variables|Default|Getstage5))))))))))))

(fn ConstructionScript)