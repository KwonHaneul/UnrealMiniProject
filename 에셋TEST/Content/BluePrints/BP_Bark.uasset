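; BP_Bark is a breakable target, apparently a gourd (박), that bursts open after five hits and moves the game to another level.
; Each hit on the Bark component prints a debug message and increments a counter.
; At the threshold it clears all widgets and plays the BarkOpen timeline, cumulatively offsetting Sphere1 along Z.
; The timeline's update also runs delays that reveal Cube, then call ChangeLevel on CatDogGameInstance.
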(event OnComponentHit(bark)
  (params (HitComponent :type Primitive%20Component%20Object%20Reference) (OtherActor :type Actor%20Object%20Reference) (OtherComp :type Primitive%20Component%20Object%20Reference) (NormalImpulse :type Vector :default "0, 0, 0") (Hit :type Hit%20Result%20Structure%20%28by%20ref%29))
  (bind _sphere1 (Variables|Default|GetSphere1))
  (Development|PrintString "Hello")
  (bind _output_get (Variables|Default|Setcount (+ (Variables|Default|Getcount) 1)))
  (if (>= _output_get 5)
    (Viewport|RemoveAllWidgets)
    ;[1 1 1] 박터지는중
    (Variables|Default|Setint_location (.location (Transformation|GetRelativeTransform (Variables|Default|GetSphere1))))
    (bind _새_트랙_1 (Timeline|Bark%20Open Play)
      (:Update
        (Utilities|FlowControl|Sequence
          (:then_0
            (Utilities|FlowControl|Delay 1.0)
            (Rendering|SetVisibility (Variables|Default|GetCube) true true)
            (Utilities|FlowControl|Delay 2.0)
            (Default|ChangeLevel (.AsCat%20Dog%20Game%20Instance (Utilities|Casting|CastToCatDogGameInstance (Game|GetGameInstance))) "NewEnumerator10"))
          (:then_1
            (Transformation|SetRelativeLocation _sphere1 (+ (Math|Vector|MakeVector 0.0 0.0 _새_트랙_1) (.location (Transformation|GetRelativeTransform _sphere1))) false false)))))))

(event Collision|EventActorBeginOverlap
  (params (OtherActor :type Actor%20Object%20Reference)))

(event EventTick
  (params (DeltaSeconds :type Float%20%28single-precision%29)))

(fn ConstructionScript)